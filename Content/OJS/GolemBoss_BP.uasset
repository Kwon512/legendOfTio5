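; Golem boss enemy pawn that roams, attacks pawns it sees and dies when health runs out.
; Roam loops through random reachable points; pawn sensing stores a target, which it approaches when in range to play an attack montage, then resumes roaming.
; Tick drives the chase check, turns the health bar widget toward the player and updates its fill, and destroys the boss shortly after health reaches zero.
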(event `self.ReceiveTick`
  (params (DeltaSeconds :type "Float (single-precision)"))
  ;[1 1 1] Tick Event
  (`self.UpdatePawnChase`)
  (`self.updateHeathBar`)
  (`self.CheckHealth`))

(event `self.ReceiveBeginPlay`
  ;[1 1 1] begin Play
  (`self.Roam`))

(event `Roam`
  ;[1 1 1] Roam
  (if (`self.isDead`)
    _
    (elif (`self.isRoaming`)
      _
      (elif (not (`self.isAttacking`))
        (set `self.isRoaming` true)
        (`|AIMoveTo` self (`NavigationSystemV1.K2_GetRandomReachablePointInRadius` (`self.K2_GetActorLocation`) 2500.0 null null) null 250.0
          (:`OnSuccess`
            _)
          (:`OnFail`
            _))
        (`KismetSystemLibrary.Delay` 3.0)
        (set `self.isRoaming` false)
        (`self.Roam`)))))

(event `self.PawnSensing.OnSeePawn`
  (params (Pawn :type "Pawn Object Reference"))
  ;[1 1 1] event - see pawn
  (set `self.chasingPawn` Pawn))

(event `UpdatePawnChase`
  ;[1 1 1] update Pawn Chase
  (`/Engine/EditorBlueprintResources/StandardMacros.IsValid` (`self.chasingPawn`)
    (:`Is Valid`
      (if (< (`KismetMathLibrary.Vector_Distance` (`self.K2_GetActorLocation` (`self.chasingPawn`)) (`self.K2_GetActorLocation`)) 2500.0)
        (if (`self.isDead`)
          _
          (elif (not (`self.isAttacking`))
            (set `self.isAttacking` true)
            (`Controller.StopMovement` (`AIBlueprintHelperLibrary.GetAIController` self))
            (`|AIMoveTo` self (0.0 0.0 0.0) (`self.chasingPawn`) 500.0
              (:`OnSuccess`
                (bind _returnvalue (`self.PlayAnimMontage` "/Game/OJS/boosAttack_Montage.boosAttack_Montage"))
                (`KismetSystemLibrary.Delay` _returnvalue))
              (:`OnFail`
                _))
            (set `self.isAttacking` false)
            (`self.Roam`)))))
    (:`Is Not Valid`
      (`self.Roam`))))

(event `updateHeathBar`
  ;[1 1 1] update Healthbar
  (`SceneComponent.K2_SetWorldRotation` (`self.HealthBar`) (`KismetMathLibrary.FindLookAtRotation` (`self.K2_GetActorLocation`) (`self.K2_GetActorLocation` (`GameplayStatics.GetPlayerCharacter` 0))) false false)
  (bind _asheath_bar (cast `/Game/OJS/HeathBar` (`WidgetComponent.GetWidget` (`self.HealthBar`))))
  (`ProgressBar.SetPercent` (`/Game/OJS/HeathBar.ProgressBar_9` _asheath_bar) (/ (`self.Health`) (`self.MaxHeath`))))

(event `CheckHealth`
  ;[1 1 1] Check Health  Death
  (if (<= (`self.Health`) 0)
    (set `self.isDead` true)
    (`Controller.StopMovement` (`AIBlueprintHelperLibrary.GetAIController` self))
    (`KismetSystemLibrary.Delay` 1.0)
    (`self.K2_DestroyActor`)))

(fn `NewFunction`)

(fn `UserConstructionScript`)